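; Game mode for a REST API demo that tracks player time and progress through Blue, Yellow and Red stages.
; A looping one-second timer, started and stopped by events, increments and prints the counter of the stage set in the stage selector.
; IncrementStageCompletion adds to the just-finished stage's attempt count in API_Info_GameInstance, inferred from the current selector value.
; OnPlayerKilled unpossesses the pawn and restarts the player.
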(event `SetTimer`
  (bind _returnvalue (`KismetSystemLibrary.K2_SetTimer` null "Increment" 1.0 true)))

(event `StopTimer`
  (`KismetSystemLibrary.K2_ClearAndInvalidateTimerHandle` (stale `SetTimer` _returnvalue)))

(event `self.ReceiveBeginPlay`)

(fn `Increment`
  (switch `/Game/Blueprints/StageSelector` (`self.StageSeclector`)
    (:`NewEnumerator0`
      (bind _output_get (set `self.blueStageCounter` (+ (`self.blueStageCounter`) 1)))
      (`KismetSystemLibrary.PrintString` (`KismetStringLibrary.Conv_IntToString` _output_get)))
    (:`NewEnumerator1`
      (bind _output_get_2 (set `self.yellowStageCounter` (+ (`self.yellowStageCounter`) 1)))
      (`KismetSystemLibrary.PrintString` (`KismetStringLibrary.Conv_IntToString` _output_get_2) true true (struct :`R` 1.0 :`G` 0.84636 :`A` 1.0)))
    (:`NewEnumerator2`
      (bind _output_get_3 (set `self.redStageCounter` (+ (`self.redStageCounter`) 1)))
      (`KismetSystemLibrary.PrintString` (`KismetStringLibrary.Conv_IntToString` _output_get_3) true true (struct :`R` 1.0 :`G` 0.014949 :`A` 1.0)))))

(fn `IncrementStageCompletion`
  (bind _asapi_info_game_instance (cast `API_Info_GameInstance` (`GameplayStatics.GetGameInstance`)))
  (switch `/Game/Blueprints/StageSelector` (`self.StageSeclector`)
    (:`NewEnumerator1`
      (bind _returnvalue (`API_Info_GameInstance.GetBlueStageAttempts` _asapi_info_game_instance))
      (bind _result (`/Engine/EditorBlueprintResources/StandardMacros.IncrementInt` _returnvalue)
        (:`  `
          (`API_Info_GameInstance.SetBlueStageAttempts` _asapi_info_game_instance _result))))
    (:`NewEnumerator2`
      (bind _returnvalue_2 (`API_Info_GameInstance.GetYellowStageAttempts` _asapi_info_game_instance))
      (bind _result_2 (`/Engine/EditorBlueprintResources/StandardMacros.IncrementInt` _returnvalue_2)
        (:`  `
          (`API_Info_GameInstance.SetYellowStageAttempts` _asapi_info_game_instance _result_2))))
    (:`NewEnumerator3`
      (bind _returnvalue_3 (`API_Info_GameInstance.GetRedStageAttempts` _asapi_info_game_instance))
      (bind _result_3 (`/Engine/EditorBlueprintResources/StandardMacros.IncrementInt` _returnvalue_3)
        (:`  `
          (`API_Info_GameInstance.SetRedStageAttempts` _asapi_info_game_instance _result_3))))))

(fn `OnPlayerKilled`
  (params (Player :type "Character Object Reference"))
  (locals (Controller :type "Controller Object Reference"))
  (bind _output_get (set `local.Controller` (`Pawn.GetController` Player)))
  (`Controller.UnPossess` _output_get)
  (`self.RestartPlayer` (`local.Controller`)))

(fn `UserConstructionScript`)
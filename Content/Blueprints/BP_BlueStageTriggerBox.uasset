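; BP_BlueStageTriggerBox is a one-shot trigger volume that marks a stage completion when the third-person player character enters it.
; On overlap it stops the player controller's periodic database save, then calls the REST API demo game mode to set its timer and increment stage completion.
; It then starts a sliding door moving up and destroys itself.
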(event `self.CollisionComponent.OnComponentBeginOverlap`
  (params (OverlappedComponent :type "PrimitiveComponent Object Reference") (OtherActor :type "Actor Object Reference") (OtherComp :type "PrimitiveComponent Object Reference") (OtherBodyIndex :type Integer) (bFromSweep :type Boolean) (SweepResult :type "HitResult Structure (by ref)"))
  (cast `/Game/ThirdPersonCPP/Blueprints/ThirdPersonCharacter` OtherActor)
  (bind _asdemo_player_controller (cast `DemoPlayerController` (`GameplayStatics.GetPlayerController` 0)))
  ;[1 1 1] Stop player data from saving to the database every 5 seconds
  (`DemoPlayerController.SaveDataRepeater` _asdemo_player_controller false)
  (bind _asbp_my_rest_api_demo_game_mode (cast `/Game/Blueprints/BP_MyREST_API_DemoGameMode` (`GameplayStatics.GetGameMode`)))
  (`/Game/Blueprints/BP_MyREST_API_DemoGameMode.SetTimer` _asbp_my_rest_api_demo_game_mode)
  (`/Game/Blueprints/BP_MyREST_API_DemoGameMode.IncrementStageCompletion` _asbp_my_rest_api_demo_game_mode)
  (`/Game/Blueprints/BP_SlidingDoor.Start Sliding Up` (`self.SlidingDoor`))
  (`self.K2_DestroyActor`))

(fn `UserConstructionScript`)
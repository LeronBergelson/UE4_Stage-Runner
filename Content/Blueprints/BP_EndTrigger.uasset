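; BP_EndTrigger is the finish-line trigger of a timed, staged course in a REST API demo game.
; When a ThirdPersonCharacter overlaps its collision component, it flags the end as reached, then sets the game mode's stage selector, stops the timer and increments stage completion.
; It passes the blue, yellow and red stage times to the DemoPlayerController, enables and triggers saving, then destroys itself.
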(event `self.CollisionComponent.OnComponentBeginOverlap`
  (params (OverlappedComponent :type "PrimitiveComponent Object Reference") (OtherActor :type "Actor Object Reference") (OtherComp :type "PrimitiveComponent Object Reference") (OtherBodyIndex :type Integer) (bFromSweep :type Boolean) (SweepResult :type "HitResult Structure (by ref)"))
  (bind _asthird_person_character (cast `/Game/ThirdPersonCPP/Blueprints/ThirdPersonCharacter` OtherActor))
  (bind _asbp_my_rest_api_demo_game_mode (cast `/Game/Blueprints/BP_MyREST_API_DemoGameMode` (`GameplayStatics.GetGameMode`)))
  (set `/Game/Blueprints/BP_MyREST_API_DemoGameMode.StageSeclector` "NewEnumerator3" _asbp_my_rest_api_demo_game_mode)
  (`REST_API_DemoCharacter.SetDidReachEnd` _asthird_person_character true)
  (`/Game/Blueprints/BP_MyREST_API_DemoGameMode.StopTimer` _asbp_my_rest_api_demo_game_mode)
  (`/Game/Blueprints/BP_MyREST_API_DemoGameMode.IncrementStageCompletion` _asbp_my_rest_api_demo_game_mode)
  (bind _asdemo_player_controller (cast `DemoPlayerController` (`GameplayStatics.GetPlayerController` 0)))
  (`DemoPlayerController.SaveCourseData` _asdemo_player_controller (`/Game/Blueprints/BP_MyREST_API_DemoGameMode.blueStageCounter` _asbp_my_rest_api_demo_game_mode) (`/Game/Blueprints/BP_MyREST_API_DemoGameMode.yellowStageCounter` _asbp_my_rest_api_demo_game_mode) (`/Game/Blueprints/BP_MyREST_API_DemoGameMode.redStageCounter` _asbp_my_rest_api_demo_game_mode))
  (`DemoPlayerController.SetCanSaveData` _asdemo_player_controller true)
  (`DemoPlayerController.SaveData` _asdemo_player_controller)
  (`self.K2_DestroyActor`))

(fn `UserConstructionScript`)